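; Player-controllable tank Blueprint that wires up turret, barrel, track movement, camera and firing.
; BeginPlay registers turret and barrel references and initializes TankMovement with left and right tracks deliberately or accidentally crossed.
; Axis inputs rotate the azimuth gimbal and spring arm separately and send movement intents to TankMovement, while Fire calls the firing function.
; The construction script assigns part meshes and sets twelve spawn points to SprungWheel_BP.
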(event `self.ReceiveBeginPlay`
  (`self.SetTurretReference` (`self.Turret`))
  (`self.SetBarrelReference` (`self.Barrel`))
  (`TankMovementComponent.Initialize` (`self.TankMovement`) (`self.RightTrack`) (`self.LeftTrack`)))

(event `InputAxis|AzimuthalRotation`
  (params (AxisValue :type "Float (single-precision)"))
  ;[1 1 1] AxisInput
  (`SceneComponent.K2_AddLocalRotation` (`self.AzimuthGimbal`) (`KismetMathLibrary.MakeRotator` 0.0 0.0 AxisValue) false false))

(event `InputAxis|MoveForwardBackward`
  (params (AxisValue :type "Float (single-precision)"))
  ;[1 1 1] Input- Movement (WASD)
  (`TankMovementComponent.IntendMoveForward` (`self.TankMovement`) AxisValue))

(event `InputAxis|MoveLeftRight`
  (params (AxisValue :type "Float (single-precision)"))
  ;[1 1 1] Input- Movement (WASD)
  (`TankMovementComponent.IntendTakeTurn` (`self.TankMovement`) AxisValue))

(event `InputAxis|AltitudeRotation`
  (params (AxisValue :type "Float (single-precision)"))
  ;[1 1 1] AxisInput
  (`SceneComponent.K2_AddLocalRotation` (`self.SpringArm`) (`KismetMathLibrary.MakeRotator` 0.0 AxisValue) false false))

(event `InputAction|Fire`
  (params (Key :type "Key Structure"))
  ;[1 1 1] AxisInput
  (:`Pressed`
    (`self.Fire`)))

(fn `UserConstructionScript`
  (`StaticMeshComponent.SetStaticMesh` (`self.LeftTrack`) "/Game/TankParts/tank_fbx_Track.tank_fbx_Track")
  (`StaticMeshComponent.SetStaticMesh` (`self.RightTrack`) "/Game/TankParts/tank_fbx_Track.tank_fbx_Track")
  (`StaticMeshComponent.SetStaticMesh` (`self.Turret`) "/Game/TankParts/tank_fbx_Turret.tank_fbx_Turret")
  (`StaticMeshComponent.SetStaticMesh` (`self.Barrel`) "/Game/TankParts/tank_fbx_Barrel.tank_fbx_Barrel")
  (bind _output_get (set `SpawnPoint.SpawnClass` "/Game/TankParts/SprungWheel_BP.SprungWheel_BP_C" (`self.SpawnPoint`)))
  (bind _output_get_2 (set `SpawnPoint.SpawnClass` _output_get (`self.SpawnPoint1`)))
  (bind _output_get_3 (set `SpawnPoint.SpawnClass` _output_get_2 (`self.SpawnPoint2`)))
  (bind _output_get_4 (set `SpawnPoint.SpawnClass` _output_get_3 (`self.SpawnPoint3`)))
  (bind _output_get_5 (set `SpawnPoint.SpawnClass` _output_get_4 (`self.SpawnPoint6`)))
  (bind _output_get_6 (set `SpawnPoint.SpawnClass` _output_get_5 (`self.SpawnPoint7`)))
  (bind _output_get_7 (set `SpawnPoint.SpawnClass` _output_get_6 (`self.SpawnPoint8`)))
  (bind _output_get_8 (set `SpawnPoint.SpawnClass` _output_get_7 (`self.SpawnPoint9`)))
  (bind _output_get_9 (set `SpawnPoint.SpawnClass` _output_get_8 (`self.SpawnPoint4`)))
  (bind _output_get_10 (set `SpawnPoint.SpawnClass` _output_get_9 (`self.SpawnPoint10`)))
  (bind _output_get_11 (set `SpawnPoint.SpawnClass` _output_get_10 (`self.SpawnPoint11`)))
  (set `SpawnPoint.SpawnClass` _output_get_11 (`self.SpawnPoint5`)))